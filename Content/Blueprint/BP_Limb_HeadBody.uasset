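; BP_Limb_HeadBody is a limb Blueprint for a head-body part that can be used, repaired and damaged.
; Its Use function passes the default per-round overheat value through PassOverheat and prints a debug message.
; Keyboard shortcuts trigger Fix, Use and TakeDamage directly with fixed amounts, apparently for testing.
; BeginPlay, overlap and Tick are left as disabled parent-call stubs.
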(event EventBeginPlay
  (|CallParentFunction) ; This node is disabled and will not be called.\nDrag off pins to build functionality.
)

(event Collision|EventActorBeginOverlap
  (params (OtherActor :type Actor%20Object%20Reference))
  (|CallParentFunction OtherActor) ; This node is disabled and will not be called.\nDrag off pins to build functionality.
)

(event EventTick
  (params (DeltaSeconds :type Float%20%28single-precision%29))
  (|CallParentFunction DeltaSeconds) ; This node is disabled and will not be called.\nDrag off pins to build functionality.
)

(event Input|KeyboardEvents|S
  (params (Key :type Key%20Structure :default "None"))
  (:Pressed
    (CallFunction|Use)))

(event Input|KeyboardEvents|X
  (params (Key :type Key%20Structure :default "None"))
  (:Pressed
    (CallFunction|TakeDamage 5.0)))

(event Input|KeyboardEvents|Z
  (params (Key :type Key%20Structure :default "None"))
  (:Pressed
    (CallFunction|Fix 1e+01)))

(fn ConstructionScript
  (|CallParentFunction))

(fn Use
  (CallFunction|PassOverheat (Variables|Default|GetdefaultOverheatRound))
  (Development|PrintString "ça use "))