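; BP_Limb_RightArm is a right-arm limb Blueprint whose Use action passes its default per-round overheat and prints a right-arm attack message.
; The attack itself is only that debug print.
; Keyboard events serve as test hooks: Q triggers Use, A calls Fix, W calls TakeDamage and K prints a string.
; BeginPlay, overlap and Tick are disabled stubs, and construction only calls the parent.
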(event EventBeginPlay
  (|CallParentFunction) ; This node is disabled and will not be called.\nDrag off pins to build functionality.
)

(event Collision|EventActorBeginOverlap
  (params (OtherActor :type Actor%20Object%20Reference))
  (|CallParentFunction OtherActor) ; This node is disabled and will not be called.\nDrag off pins to build functionality.
)

(event EventTick
  (params (DeltaSeconds :type Float%20%28single-precision%29))
  (|CallParentFunction DeltaSeconds) ; This node is disabled and will not be called.\nDrag off pins to build functionality.
)

(event Input|KeyboardEvents|Q
  (params (Key :type Key%20Structure :default "None"))
  (:Pressed
    (CallFunction|Use)))

(event Input|KeyboardEvents|W
  (params (Key :type Key%20Structure :default "None"))
  (:Pressed
    (CallFunction|TakeDamage 5.0)))

(event Input|KeyboardEvents|A
  (params (Key :type Key%20Structure :default "None"))
  (:Pressed
    (CallFunction|Fix 1e+01)))

(event Input|KeyboardEvents|K
  (params (Key :type Key%20Structure :default "None"))
  (:Pressed
    (Development|PrintString "Yo?")))

(fn ConstructionScript
  (|CallParentFunction))

(fn Use
  (CallFunction|PassOverheat (Variables|Default|GetdefaultOverheatRound))
  (Development|PrintString "Attack Bras Droit !"))