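; BPC_Robot1 is a player robot for turn-based fights, built from four BP_Limb child actors: head, both arms and legs.
; BeginPlay sets each limb's life and creates the WBP_Round fight UI.
; GetAction queues action and limb picks until the turn quota is met, then notifies ManagerTurn.
; ExecuteActionInTurn runs the queue, where block and dodge only print and Fix repairs limbs (leftArm targets RightArm), then clears it.
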(event Custom|GetAction
  (params (ActionSelect :type Name) (MemberSelect :type String))
  (if (not (Variables|Default|GetFInishPrep))
    (Utilities|Array|Add (Variables|Default|GetListActionTurn) ActionSelect)
    (Utilities|Array|Add (Variables|Default|GetListMemberTurn) MemberSelect)
    (Default|UpdateDisplayActionChoice (Variables|Default|GetUIFight) (- (Utilities|Array|Length (Variables|Default|GetListActionTurn)) 1) ActionSelect)
    (if (>= (Utilities|Array|Length (Variables|Default|GetListActionTurn)) (Variables|Default|GetNumberActionInTurn))
      (Variables|Default|SetFInishPrep true)
      (Default|PlayerFinishPrep (Variables|Default|GetManagerTurn) self))))

(event Custom|ExecuteActionInTurn
  (for (_array_element _array_index) (Variables|Default|GetListActionTurn)
    (if (== _array_element "Bloque")
      (Development|PrintString "Bloque")
      (Utilities|FlowControl|Delay 2.0 :!label _label)
      (elif (== _array_element "Dodge")
        (Development|PrintString "dodge")
        (goto _label)
        (elif (== _array_element "Fix")
          (Utilities|FlowControl|Sequence
            (:then_0
              (if (== (Utilities|Array|Get(acopy) (Variables|Default|GetListMemberTurn) _array_index) "Head")
                (bind _asbp_limb (Utilities|Casting|CastToBP_Limb (Variables|/Script/Engine.ChildActorComponent|GetChildActor (Variables|Default|GetHead))))
                (Default|Fix _asbp_limb 1e+01)
                (goto _label)))
            (:then_1
              (if (== (Utilities|Array|Get(acopy) (Variables|Default|GetListMemberTurn) _array_index) "Legs")
                (bind _asbp_limb_2 (Utilities|Casting|CastToBP_Limb (Variables|/Script/Engine.ChildActorComponent|GetChildActor (Variables|Default|GetLegs))))
                (Default|Fix _asbp_limb_2 1e+01)
                (goto _label)))
            (:then_2
              (if (== (Utilities|Array|Get(acopy) (Variables|Default|GetListMemberTurn) _array_index) "RightArm")
                (bind _asbp_limb_3 (Utilities|Casting|CastToBP_Limb (Variables|/Script/Engine.ChildActorComponent|GetChildActor (Variables|Default|GetRightArm))))
                (Default|Fix _asbp_limb_3 1e+01)
                (goto _label)))
            (:then_3
              (if (== (Utilities|Array|Get(acopy) (Variables|Default|GetListMemberTurn) _array_index) "leftArm")
                (bind _asbp_limb_4 (Utilities|Casting|CastToBP_Limb (Variables|/Script/Engine.ChildActorComponent|GetChildActor (Variables|Default|GetRightArm))))
                (Default|Fix _asbp_limb_4 1e+01)
                (goto _label))))))))
  (Utilities|Array|Clear (Variables|Default|GetListActionTurn))
  (Utilities|Array|Clear (Variables|Default|GetListMemberTurn))
  (for _array_element_2 (Variables|/Game/Ui/WBP_Round.WBP_Round_C|GetListActionChoice (Variables|Default|GetUIFight))
    (Widget|SetVisibility _array_element_2 "Hidden")))

(event EventBeginPlay
  (Utilities|FlowControl|Sequence
    (:then_0
      (bind _asbp_limb (Utilities|Casting|CastToBP_Limb (Variables|/Script/Engine.ChildActorComponent|GetChildActor (Variables|Default|GetHead))))
      (bind _output_get (Variables|/Game/Blueprint/BP_Limb.BP_Limb_C|SetInitialLife _asbp_limb (Variables|Default|GetLifeHeadTors)))
      (Variables|/Game/Blueprint/BP_Limb.BP_Limb_C|Setlife _asbp_limb _output_get))
    (:then_1
      (bind _asbp_limb_2 (Utilities|Casting|CastToBP_Limb (Variables|/Script/Engine.ChildActorComponent|GetChildActor (Variables|Default|GetRightArm))))
      (bind _output_get_2 (Variables|/Game/Blueprint/BP_Limb.BP_Limb_C|SetInitialLife _asbp_limb_2 (Variables|Default|GetLifeRightArm)))
      (Variables|/Game/Blueprint/BP_Limb.BP_Limb_C|Setlife _asbp_limb_2 _output_get_2))
    (:then_2
      (bind _asbp_limb_3 (Utilities|Casting|CastToBP_Limb (Variables|/Script/Engine.ChildActorComponent|GetChildActor (Variables|Default|GetleftArm))))
      (bind _output_get_3 (Variables|/Game/Blueprint/BP_Limb.BP_Limb_C|SetInitialLife _asbp_limb_3 (Variables|Default|GetLifeLeftArm)))
      (Variables|/Game/Blueprint/BP_Limb.BP_Limb_C|Setlife _asbp_limb_3 _output_get_3))
    (:then_3
      (bind _asbp_limb_4 (Utilities|Casting|CastToBP_Limb (Variables|/Script/Engine.ChildActorComponent|GetChildActor (Variables|Default|GetLegs))))
      (bind _output_get_4 (Variables|/Game/Blueprint/BP_Limb.BP_Limb_C|SetInitialLife _asbp_limb_4 (Variables|Default|GetLifeLegs)))
      (Variables|/Game/Blueprint/BP_Limb.BP_Limb_C|Setlife _asbp_limb_4 _output_get_4))
    (:then_4
      (bind _returnvalue (UserInterface|CreateWidget "/Game/Ui/WBP_Round.WBP_Round_C"))
      (bind _output_get_5 (Variables|Default|SetUIFight _returnvalue))
      (UserInterface|Viewport|AddtoViewport _output_get_5 0)
      (Variables|/Game/Ui/WBP_Round.WBP_Round_C|SetPlayerAssociate (Variables|Default|GetUIFight) self))))

(fn ConstructionScript)