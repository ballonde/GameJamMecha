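; TurnSystem is a turn manager that runs two robot players through a prep phase and a series of simultaneous action steps.
; It registers itself on BPC_Robot1 actors, then waits for two prep-finished calls before starting turns.
; Each turn has both robots execute the action at the current index.
; ResolutionTurn stores both reported action/member choices, then advances the index, ending the round after ten steps.
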(event Custom|PlayerFinishPrep
  (Development|PrintString (Utilities|String|ToString(Boolean) (Variables|Default|GetPlayer1FinishCHoiceAction)))
  (if (== (Variables|Default|GetPlayer1FinishCHoiceAction) false)
    (bind _output_get (Variables|Default|SetPlayer1FinishCHoiceAction true))
    (else
      (bind _output_get_2 (Variables|Default|SetPlayer2FinishCHoiceAction true))
      (if (and _output_get _output_get_2)
        (Variables|Default|SetPlayer1FinishCHoiceAction false)
        (CallFunction|Turn)))))

(event Custom|ResolutionTurn
  (params (ActionChoice :type Name) (MemberChoice :type String) (Player :type String))
  (if (Variables|Default|GetPlayer1FinishCHoiceAction)
    (Variables|Default|SetActionChoice2 ActionChoice)
    (Variables|Default|SetMemberSelect2 MemberChoice)
    (Variables|Default|SetPlayer1FinishCHoiceAction false)
    (Variables|Default|SetPlayer2FinishCHoiceAction false)
    (bind _result (Math|Integer|IncrementInt (Variables|Default|GetIndexTurn))
      (:%20%20
        (Variables|Default|SetIndexTurn _result)
        (Development|PrintString "Resolution d'effet")
        (CallFunction|Turn)))
    (else
      (Variables|Default|SetActionChoice1 ActionChoice)
      (Variables|Default|SetMemberSelect1 MemberChoice)
      (Variables|Default|SetPlayer1FinishCHoiceAction true))))

(event Custom|Turn
  (if (>= (Variables|Default|GetIndexTurn) 10)
    (Default|EndTurn (stale _returnvalue_2))
    (Default|EndTurn (stale _returnvalue))
    (Variables|Default|SetIndexTurn 0)
    (else
      (bind _returnvalue (Actor|GetActorOfClass "/Game/Blueprint/BPC_Robot1.BPC_Robot1_C"))
      (Default|ExecuteActioninTurn _returnvalue (Variables|Default|GetIndexTurn))
      (bind _returnvalue_2 (Actor|GetActorOfClass "/Game/Blueprint/BPC_Robot2.BPC_Robot2_C"))
      (Default|ExecuteActioninTurn _returnvalue_2 (Variables|Default|GetIndexTurn)))))

(event EventBeginPlay
  (bind _outactors (Actor|GetAllActorsOfClass "/Game/Blueprint/BPC_Robot1.BPC_Robot1_C"))
  (for _array_element _outactors
    (bind _asbpc_robot_1 (Utilities|Casting|CastToBPC_Robot1 _array_element))
    (Variables|/Game/Blueprint/BPC_Robot1.BPC_Robot1_C|SetManagerTurn _asbpc_robot_1 self)))

(fn ConstructionScript)