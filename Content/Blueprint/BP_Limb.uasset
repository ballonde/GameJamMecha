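; BP_Limb is a limb with its own life pool that can take damage, be repaired and overheat.
; TakeDamage lowers Life and Fix restores it up to InitialLife, both printing French debug messages, with zero life only reported as destroyed.
; PassOverheat flags the limb as overheated, or damages it if already so, then adds to its overheat round count.
; Use is an empty stub, and BeginPlay enables player input.
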(event EventBeginPlay
  (Input|EnableInput (Game|GetPlayerController 0)))

(fn ConstructionScript)

(fn TakeDamage
  (params (nbDamage :type Float%20%28double-precision%29))
  (bind _output_get (Variables|Default|Setlife (- (Variables|Default|Getlife) nbDamage)))
  (if (<= _output_get 0.0)
    (Development|PrintString "Membre Détruit")
    (Development|PrintString (Utilities|String|ToString(Float) _output_get))
    (else
      (Development|PrintString "On Prend des dégats")
      (Development|PrintString (Utilities|String|ToString(Float) _output_get)))))

(fn Fix
  (params (nbLife :type Float%20%28double-precision%29))
  (if (> (+ nbLife (Variables|Default|Getlife)) (Variables|Default|GetInitialLife))
    (Variables|Default|Setlife (Variables|Default|GetInitialLife))
    (Development|PrintString "Ca répare au max")
    (else
      (Variables|Default|Setlife (+ nbLife (Variables|Default|Getlife)))
      (Development|PrintString "Ca répare !"))))

(fn PassOverheat
  (params (nbRound :type Integer))
  (Utilities|FlowControl|Sequence
    (:then_0
      (if (Variables|Default|GetisOverheated)
        (CallFunction|TakeDamage (Variables|Default|GetNb%20DamageOverHeath))
        (else
          (Variables|Default|SetisOverheated true))))
    (:then_1
      (Variables|Default|SetnbRoundOverheat (+ nbRound (Variables|Default|GetnbRoundOverheat))))))

(fn Use)