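; Player 2 robot for a turn-based fight, acting as a scripted opponent that always picks Dodge with Legs.
; On BeginPlay it sets the life of four BP_Limb child actors (head, arms, legs), then queues its choices.
; GetAction fills parallel action/member lists up to the turn limit, then notifies ManagerTurn.
; ExecuteActionInTurn sends queued pairs to ManagerTurn for resolution; EndTurn clears and refills the queue.
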(event Custom|GetAction
  (params (ActionSelect :type Name) (MemberSelect :type String))
  (if (not (Variables|Default|GetFInishPrep))
    (Utilities|Array|Add (Variables|Default|GetListActionTurn) ActionSelect)
    (Utilities|Array|Add (Variables|Default|GetListMemberTurn) MemberSelect)
    (if (>= (Utilities|Array|Length (Variables|Default|GetListActionTurn)) (Variables|Default|GetNumberActionInTurn))
      (Variables|Default|SetFInishPrep true)
      (Default|PlayerFinishPrep (Variables|Default|GetManagerTurn)))))

(event Custom|ChoiceTurn
  (CallFunction|GetAction "Dodge" "Legs")
  (CallFunction|GetAction "Dodge" "Legs")
  (CallFunction|GetAction "Dodge" "Legs")
  (CallFunction|GetAction "Dodge" "Legs")
  (CallFunction|GetAction "Dodge" "Legs")
  (CallFunction|GetAction "Dodge" "Legs")
  (CallFunction|GetAction "Dodge" "Legs")
  (CallFunction|GetAction "Dodge" "Legs")
  (CallFunction|GetAction "Dodge" "Legs")
  (CallFunction|GetAction "Dodge" "Legs"))

(event Custom|EndTurn
  (Utilities|Array|Clear (Variables|Default|GetListActionTurn))
  (Utilities|Array|Clear (Variables|Default|GetListMemberTurn))
  (Variables|Default|SetFInishPrep false)
  (CallFunction|ChoiceTurn))

(event Custom|ExecuteActionInTurn
  (params (Index :type Integer))
  (Default|ResolutionTurn (Variables|Default|GetManagerTurn) (Utilities|Array|Get(acopy) (Variables|Default|GetListActionTurn) Index) (Utilities|Array|Get(acopy) (Variables|Default|GetListMemberTurn) Index) "Player2"))

(event EventBeginPlay
  (Utilities|FlowControl|Sequence
    (:then_0
      (bind _asbp_limb (Utilities|Casting|CastToBP_Limb (Variables|/Script/Engine.ChildActorComponent|GetChildActor (Variables|Default|GetHead))))
      (bind _output_get (Variables|/Game/Blueprint/BP_Limb.BP_Limb_C|SetInitialLife _asbp_limb (Variables|Default|GetLifeHeadTors)))
      (Variables|/Game/Blueprint/BP_Limb.BP_Limb_C|Setlife _asbp_limb _output_get))
    (:then_1
      (bind _asbp_limb_2 (Utilities|Casting|CastToBP_Limb (Variables|/Script/Engine.ChildActorComponent|GetChildActor (Variables|Default|GetRightArm))))
      (bind _output_get_2 (Variables|/Game/Blueprint/BP_Limb.BP_Limb_C|SetInitialLife _asbp_limb_2 (Variables|Default|GetLifeRightArm)))
      (Variables|/Game/Blueprint/BP_Limb.BP_Limb_C|Setlife _asbp_limb_2 _output_get_2))
    (:then_2
      (bind _asbp_limb_3 (Utilities|Casting|CastToBP_Limb (Variables|/Script/Engine.ChildActorComponent|GetChildActor (Variables|Default|GetleftArm))))
      (bind _output_get_3 (Variables|/Game/Blueprint/BP_Limb.BP_Limb_C|SetInitialLife _asbp_limb_3 (Variables|Default|GetLifeLeftArm)))
      (Variables|/Game/Blueprint/BP_Limb.BP_Limb_C|Setlife _asbp_limb_3 _output_get_3))
    (:then_3
      (bind _asbp_limb_4 (Utilities|Casting|CastToBP_Limb (Variables|/Script/Engine.ChildActorComponent|GetChildActor (Variables|Default|GetLegs))))
      (bind _output_get_4 (Variables|/Game/Blueprint/BP_Limb.BP_Limb_C|SetInitialLife _asbp_limb_4 (Variables|Default|GetLifeLegs)))
      (Variables|/Game/Blueprint/BP_Limb.BP_Limb_C|Setlife _asbp_limb_4 _output_get_4))
    (:then_4
      (CallFunction|ChoiceTurn))))

(fn ConstructionScript)