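; BP_Mecha is the mecha Blueprint that exposes combat actions and drives their animation states.
; Events for melee attack, ranged attack, shield, repair, dodge and hit each cast the mesh's anim instance to ABP_Mecha and raise the matching boolean.
; Each flag clears after a fixed two-second Delay rather than when the animation ends.
; It holds no damage or gameplay logic, and its construction script is empty.
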(event Custom|AttackMelee
  (bind _asabp_mecha (Utilities|Casting|CastToABP_Mecha (Components|SkeletalMesh|GetAnimInstance (Variables|Character|GetMesh))))
  (Variables|/Game/Mechas/ABP_Mecha.ABP_Mecha_C|SetAttack_Melee _asabp_mecha true)
  (Utilities|FlowControl|Delay 2.0)
  (Variables|/Game/Mechas/ABP_Mecha.ABP_Mecha_C|SetAttack_Melee _asabp_mecha false))

(event Custom|Dodge
  (bind _asabp_mecha (Utilities|Casting|CastToABP_Mecha (Components|SkeletalMesh|GetAnimInstance (Variables|Character|GetMesh))))
  (Variables|/Game/Mechas/ABP_Mecha.ABP_Mecha_C|SetDodging _asabp_mecha true)
  (Utilities|FlowControl|Delay 2.0)
  (Variables|/Game/Mechas/ABP_Mecha.ABP_Mecha_C|SetDodging _asabp_mecha false))

(event Custom|Hit
  (bind _asabp_mecha (Utilities|Casting|CastToABP_Mecha (Components|SkeletalMesh|GetAnimInstance (Variables|Character|GetMesh))))
  (Variables|/Game/Mechas/ABP_Mecha.ABP_Mecha_C|SetIsHit _asabp_mecha true)
  (Utilities|FlowControl|Delay 2.0)
  (Variables|/Game/Mechas/ABP_Mecha.ABP_Mecha_C|SetIsHit _asabp_mecha false))

(event Custom|AttackRange
  (bind _asabp_mecha (Utilities|Casting|CastToABP_Mecha (Components|SkeletalMesh|GetAnimInstance (Variables|Character|GetMesh))))
  (Variables|/Game/Mechas/ABP_Mecha.ABP_Mecha_C|SetAttack_Range _asabp_mecha true)
  (Utilities|FlowControl|Delay 2.0)
  (Variables|/Game/Mechas/ABP_Mecha.ABP_Mecha_C|SetAttack_Range _asabp_mecha false))

(event Custom|Shield
  (bind _asabp_mecha (Utilities|Casting|CastToABP_Mecha (Components|SkeletalMesh|GetAnimInstance (Variables|Character|GetMesh))))
  (Variables|/Game/Mechas/ABP_Mecha.ABP_Mecha_C|SetShield _asabp_mecha true)
  (Utilities|FlowControl|Delay 2.0)
  (Variables|/Game/Mechas/ABP_Mecha.ABP_Mecha_C|SetShield _asabp_mecha false))

(event Custom|Repair
  (bind _asabp_mecha (Utilities|Casting|CastToABP_Mecha (Components|SkeletalMesh|GetAnimInstance (Variables|Character|GetMesh))))
  (Variables|/Game/Mechas/ABP_Mecha.ABP_Mecha_C|SetRepair _asabp_mecha true)
  (Utilities|FlowControl|Delay 2.0)
  (Variables|/Game/Mechas/ABP_Mecha.ABP_Mecha_C|SetRepair _asabp_mecha false))

(fn ConstructionScript)